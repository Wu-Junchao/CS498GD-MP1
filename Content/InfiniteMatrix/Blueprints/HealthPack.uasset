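; HealthPack is a timed pickup Actor that gives BP_Player one point of Health when touched.
; Tick spins the HPPack component and counts TimeToDestroy down, destroying the actor when it runs out.
; A player overlap raises Health only if below MaxHp and refreshes the HP widget text, but consumes the pack either way.
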(event `self.ReceiveTick`
  (params (DeltaSeconds :type "Float (single-precision)"))
  (`SceneComponent.K2_AddLocalRotation` (`self.HP_Pack`) (`KismetMathLibrary.MakeRotator` (* DeltaSeconds 100.0)) false false)
  (bind _output_get (set `self.TimeToDestroy` (- (`self.TimeToDestroy`) DeltaSeconds)))
  (if (<= _output_get 0.0)
    (`self.K2_DestroyActor`)))

(event `self.HP_Pack.OnComponentBeginOverlap`
  (params (OverlappedComponent :type "PrimitiveComponent Object Reference") (OtherActor :type "Actor Object Reference") (OtherComp :type "PrimitiveComponent Object Reference") (OtherBodyIndex :type Integer) (bFromSweep :type Boolean) (SweepResult :type "HitResult Structure (by ref)"))
  (bind _asbp_player (cast `/Game/InfiniteMatrix/Blueprints/BP_Player` OtherActor))
  (bind _health (`/Game/InfiniteMatrix/Blueprints/BP_Player.health` _asbp_player))
  (if (< _health (`/Game/InfiniteMatrix/Blueprints/BP_Player.MaxHp` _asbp_player))
    (bind _result (`/Engine/EditorBlueprintResources/StandardMacros.IncrementInt` _health)
      (:`  `
        (set `/Game/InfiniteMatrix/Blueprints/BP_Player.health` _result _asbp_player)
        (`/Game/InfiniteMatrix/UI/HPScore.UpdateHpText` (`/Game/InfiniteMatrix/Blueprints/BP_Player.HP_Widget` _asbp_player)))))
  (`self.K2_DestroyActor`))

(fn `UserConstructionScript`)