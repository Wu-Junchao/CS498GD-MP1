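; Enemy actor that spins its mesh on roll each tick and destroys itself when its lifetime countdown runs out.
; Overlapping a living player costs health, destroys the enemy and triggers the restart display at zero health.
; Other overlaps, except fellow enemies, also destroy it.
; Bullet hits first raise score and update the speed multiplier on the first BP_Player found, gated by that player's bullet cooldown.
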(event `self.ReceiveTick`
  (params (DeltaSeconds :type "Float (single-precision)"))
  (`SceneComponent.K2_AddLocalRotation` (`self.StaticMesh`) (`KismetMathLibrary.MakeRotator` (* DeltaSeconds 100.0)) false false)
  (bind _output_get (set `self.TimeToDestroy` (- (`self.TimeToDestroy`) DeltaSeconds)))
  (if (<= _output_get 0.0)
    (`self.K2_DestroyActor`)))

(event `self.StaticMesh.OnComponentBeginOverlap`
  (params (OverlappedComponent :type "PrimitiveComponent Object Reference") (OtherActor :type "Actor Object Reference") (OtherComp :type "PrimitiveComponent Object Reference") (OtherBodyIndex :type Integer) (bFromSweep :type Boolean) (SweepResult :type "HitResult Structure (by ref)"))
  (bind _asbp_player (cast `/Game/InfiniteMatrix/Blueprints/BP_Player` OtherActor)
    (:`then`
      (if (not (`/Game/InfiniteMatrix/Blueprints/BP_Player.IsDead` _asbp_player))
        (bind _result (`/Engine/EditorBlueprintResources/StandardMacros.DecrementInt` (`/Game/InfiniteMatrix/Blueprints/BP_Player.health` _asbp_player))
          (:`  `
            (bind _output_get (set `/Game/InfiniteMatrix/Blueprints/BP_Player.health` _result _asbp_player))
            (`/Game/InfiniteMatrix/UI/HPScore.UpdateHpText` (`/Game/InfiniteMatrix/Blueprints/BP_Player.HP_Widget` _asbp_player))
            (`self.K2_DestroyActor`)
            (if (== _output_get 0)
              (set `/Game/InfiniteMatrix/Blueprints/BP_Player.IsDead` true _asbp_player)
              (`/Game/InfiniteMatrix/Blueprints/BP_Player.DisplayRestart` _asbp_player))))))
    (:`CastFailed`
      (cast `/Game/InfiniteMatrix/Blueprints/Enemy` OtherActor
        (:`CastFailed`
          (bind _asbullet (cast `/Game/InfiniteMatrix/Blueprints/Bullet` OtherActor)
            (:`then`
              (`self.BulletOverlap` _asbullet))
            (:`CastFailed`
              _))
          (`self.K2_DestroyActor`))))))

(fn `BulletOverlap`
  (params (bullet :type "/Game/InfiniteMatrix/Blueprints/Bullet Object Reference"))
  (bind _outactors (`GameplayStatics.GetAllActorsOfClass` "/Game/InfiniteMatrix/Blueprints/BP_Player.BP_Player_C"))
  (bind _output (`|GetArrayItem` _outactors))
  (if (<= (`/Game/InfiniteMatrix/Blueprints/BP_Player.Bullet_CD` _output) 0.0)
    (set `/Game/InfiniteMatrix/Blueprints/BP_Player.Bullet_CD` (`/Game/InfiniteMatrix/Blueprints/BP_Player.Bullet_CD_Max` _output) _output)
    (bind _result (`/Engine/EditorBlueprintResources/StandardMacros.IncrementFloat` (`/Game/InfiniteMatrix/Blueprints/BP_Player.Score` _output))
      (:`  `
        (set `/Game/InfiniteMatrix/Blueprints/BP_Player.Score` _result _output)
        (`/Game/InfiniteMatrix/Blueprints/BP_Player.UpdateSpeedMulti` _output)
        (`/Game/InfiniteMatrix/UI/HPScore.UpdateScoreText` (`/Game/InfiniteMatrix/Blueprints/BP_Player.HP_Widget` _output))))))

(fn `UserConstructionScript`)