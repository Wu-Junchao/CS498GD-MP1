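; Bullet is a projectile actor that flies along the world X axis and destroys itself on overlap or when its lifetime runs out.
; Each tick it counts down its remaining time and sweeps forward at one and a half times the player's forward speed, scaled by the player's speed multiplier.
; The player reference comes from an actor search, run only while that reference is invalid.
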(event `self.ReceiveTick`
  (params (DeltaSeconds :type "Float (single-precision)"))
  (bind _bp_player (`self.BP_Player`))
  (`/Engine/EditorBlueprintResources/StandardMacros.IsValid` (`self.BP_Player`)
    (:`Is Valid`
      _)
    (:`Is Not Valid`
      (bind _outactors (`GameplayStatics.GetAllActorsOfClass` "/Game/InfiniteMatrix/Blueprints/BP_Player.BP_Player_C"))
      (set `self.BP_Player` (`|GetArrayItem` _outactors))))
  (bind _output_get (set `self.Time Remains` (- (`self.Time Remains`) DeltaSeconds)))
  (if (<= _output_get 0.0)
    (`self.K2_DestroyActor`)
    (else
      (`self.K2_AddActorWorldOffset` (`KismetMathLibrary.MakeVector` (* (* DeltaSeconds (* (`/Game/InfiniteMatrix/Blueprints/BP_Player.ForwardSpeed` _bp_player) 1.5)) (`/Game/InfiniteMatrix/Blueprints/BP_Player.SpeedMulti` _bp_player))) true))))

(event `self.StaticMesh.OnComponentBeginOverlap`
  (params (OverlappedComponent :type "PrimitiveComponent Object Reference") (OtherActor :type "Actor Object Reference") (OtherComp :type "PrimitiveComponent Object Reference") (OtherBodyIndex :type Integer) (bFromSweep :type Boolean) (SweepResult :type "HitResult Structure (by ref)"))
  (`self.K2_DestroyActor`))

(fn `UserConstructionScript`)