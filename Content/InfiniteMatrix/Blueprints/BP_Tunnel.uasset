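; Endless-runner tunnel segment with a rotating holed wall that the player must pass through.
; Crossing the trigger zone has TunnelSpawner spawn another tunnel and destroys this one, awarding score and updating speed only if the wall was not hit.
; Wall hits cost one health and show restart at zero.
; RandomizeWall picks hole mesh and roll, while Tick looks up the player to swap low/high-HP materials at one-third health.
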(event `self.ReceiveTick`
  (params (DeltaSeconds :type "Float (single-precision)"))
  (`SceneComponent.K2_AddLocalRotation` (`self.WallMesh`) (`KismetMathLibrary.MakeRotator` (* DeltaSeconds (`self.RotateSpeed`))) false false)
  (bind _outactors (`GameplayStatics.GetAllActorsOfClass` "/Game/InfiniteMatrix/Blueprints/BP_Player.BP_Player_C"))
  (bind _output (`|GetArrayItem` _outactors))
  (if (<= (`KismetMathLibrary.Conv_IntToDouble` (`/Game/InfiniteMatrix/Blueprints/BP_Player.health` _output)) (/ (`KismetMathLibrary.Conv_IntToDouble` (`/Game/InfiniteMatrix/Blueprints/BP_Player.MaxHp` _output)) 3.0))
    (`self.LowHP_Scene`)
    (else
      (`self.HighHP_Scene`))))

(event `self.TriggerZone.OnComponentBeginOverlap`
  (params (OverlappedComponent :type "PrimitiveComponent Object Reference") (OtherActor :type "Actor Object Reference") (OtherComp :type "PrimitiveComponent Object Reference") (OtherBodyIndex :type Integer) (bFromSweep :type Boolean) (SweepResult :type "HitResult Structure (by ref)"))
  (bind _asbp_player (cast `/Game/InfiniteMatrix/Blueprints/BP_Player` OtherActor))
  (`/Game/InfiniteMatrix/Blueprints/BP_TunnelSpawner.SpawnTunnelAtSpawnPoint` (`self.TunnelSpawner`))
  (if (not (`self.flg`))
    (bind _result (`/Engine/EditorBlueprintResources/StandardMacros.IncrementFloat` (`/Game/InfiniteMatrix/Blueprints/BP_Player.Score` _asbp_player))
      (:`  `
        (set `/Game/InfiniteMatrix/Blueprints/BP_Player.Score` _result _asbp_player)
        (`/Game/InfiniteMatrix/Blueprints/BP_Player.UpdateSpeedMulti` _asbp_player)
        (`/Game/InfiniteMatrix/UI/HPScore.UpdateScoreText` (`/Game/InfiniteMatrix/Blueprints/BP_Player.HP_Widget` _asbp_player)))))
  (`self.K2_DestroyActor`))

(event `self.WallMesh.OnComponentBeginOverlap`
  (params (OverlappedComponent :type "PrimitiveComponent Object Reference") (OtherActor :type "Actor Object Reference") (OtherComp :type "PrimitiveComponent Object Reference") (OtherBodyIndex :type Integer) (bFromSweep :type Boolean) (SweepResult :type "HitResult Structure (by ref)"))
  (bind _asbp_player (cast `/Game/InfiniteMatrix/Blueprints/BP_Player` OtherActor))
  (if (not (`/Game/InfiniteMatrix/Blueprints/BP_Player.IsDead` _asbp_player))
    (bind _result (`/Engine/EditorBlueprintResources/StandardMacros.DecrementInt` (`/Game/InfiniteMatrix/Blueprints/BP_Player.health` _asbp_player))
      (:`  `
        (bind _output_get (set `/Game/InfiniteMatrix/Blueprints/BP_Player.health` _result _asbp_player))
        (`/Game/InfiniteMatrix/UI/HPScore.UpdateHpText` (`/Game/InfiniteMatrix/Blueprints/BP_Player.HP_Widget` _asbp_player))
        (set `self.flg` true)
        (if (== _output_get 0)
          (set `/Game/InfiniteMatrix/Blueprints/BP_Player.IsDead` true _asbp_player)
          (`/Game/InfiniteMatrix/Blueprints/BP_Player.DisplayRestart` _asbp_player))))))

(fn `HighHP_Scene`
  (`PrimitiveComponent.SetMaterial` (`self.StaticMeshComponent`) 0 "/Game/InfiniteMatrix/Materials/MI_Tunnel.MI_Tunnel")
  (`PrimitiveComponent.SetMaterial` (`self.WallMesh`) 0 "/Game/InfiniteMatrix/Materials/MI_Hole.MI_Hole"))

(fn `LowHP_Scene`
  (`PrimitiveComponent.SetMaterial` (`self.StaticMeshComponent`) 0 "/Game/InfiniteMatrix/Materials/Tunnel_lowHP.Tunnel_lowHP")
  (`PrimitiveComponent.SetMaterial` (`self.WallMesh`) 0 "/Game/InfiniteMatrix/Materials/B.B"))

(fn `RandomizeWall`
  (`StaticMeshComponent.SetStaticMesh` (`self.WallMesh`) (select `int` (`KismetMathLibrary.RandomIntegerInRange` 0 3) :`0` "/Game/InfiniteMatrix/Meshes/SM_Hole_01.SM_Hole_01" :`1` "/Game/InfiniteMatrix/Meshes/SM_Hole_02.SM_Hole_02" :`2` "/Game/InfiniteMatrix/Meshes/SM_Hole_03.SM_Hole_03" :`3` "/Game/InfiniteMatrix/Meshes/SM_Hole_04.SM_Hole_04" :!type "StaticMesh Object Reference"))
  (`SceneComponent.K2_AddLocalRotation` (`self.WallMesh`) (`KismetMathLibrary.MakeRotator` (`KismetMathLibrary.Conv_IntToDouble` (`KismetMathLibrary.RandomIntegerInRange` 0 300))) false false))

(fn `UserConstructionScript`)